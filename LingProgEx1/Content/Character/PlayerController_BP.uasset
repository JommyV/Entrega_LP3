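; Player controller that handles character input for moving, looking, jumping and interacting with nearby objects such as doors.
; BeginPlay adds the character Enhanced Input mapping context.
; Move and Look act on the controlled pawn relative to its control rotation, while Jump calls a stored character reference.
; OpenDoor scans actors overlapping that character's capsule and sends InteractMessage to the first one implementing InteractInterface_BP.
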(event `self.ReceiveBeginPlay`
  (`EnhancedInputSubsystemInterface.AddMappingContext` (subsystem `EnhancedInputLocalPlayerSubsystem`) "/Game/Character/Input/InputContextCharacter.InputContextCharacter" 0 (struct)))

(event `EnhancedInput|/Game/Character/Input/Move`
  (params (ActionValue :type "Vector2D Structure") (ElapsedSeconds :type "Float (double-precision)") (TriggeredSeconds :type "Float (double-precision)") (InputAction :type "InputAction Object Reference" :default "/Game/Character/Input/Move.Move"))
  (bind (_x _y) (`KismetMathLibrary.BreakVector2D` ActionValue))
  (bind _returnvalue (`Pawn.GetControlRotation` (`self.K2_GetPawn`)))
  (:`Triggered`
    (`Pawn.AddMovementInput` (`self.K2_GetPawn`) (+ (* (`KismetMathLibrary.GetForwardVector` _returnvalue) _x) (* (`KismetMathLibrary.GetRightVector` _returnvalue) _y)) 1.0 false)))

(event `EnhancedInput|/Game/Character/Input/Jump`
  (params (ActionValue :type Boolean) (ElapsedSeconds :type "Float (double-precision)") (TriggeredSeconds :type "Float (double-precision)") (InputAction :type "InputAction Object Reference" :default "/Game/Character/Input/Jump.Jump"))
  (:`Triggered`
    (`Character.Jump` (`self.CharReference`))))

(event `EnhancedInput|/Game/Character/Input/OpenDoor`
  (params (ActionValue :type Boolean) (ElapsedSeconds :type "Float (double-precision)") (TriggeredSeconds :type "Float (double-precision)") (InputAction :type "InputAction Object Reference" :default "/Game/Character/Input/OpenDoor.OpenDoor"))
  (:`Triggered`
    (for _array_element (`PrimitiveComponent.GetOverlappingActors` (`Character.CapsuleComponent` (`self.CharReference`)) null)
      (if (`KismetSystemLibrary.DoesImplementInterface` _array_element "/Game/Character/Door/InteractInterface_BP.InteractInterface_BP_C")
        (message `/Game/Character/Door/InteractInterface_BP.Interact` _array_element)
        (break)))))

(event `EnhancedInput|/Game/Character/Input/Look`
  (params (ActionValue :type "Vector2D Structure") (ElapsedSeconds :type "Float (double-precision)") (TriggeredSeconds :type "Float (double-precision)") (InputAction :type "InputAction Object Reference" :default "/Game/Character/Input/Look.Look"))
  (bind _returnvalue (`self.K2_GetPawn`))
  (:`Triggered`
    (`Pawn.AddControllerYawInput` _returnvalue ActionValue_X)
    (`Pawn.AddControllerPitchInput` _returnvalue ActionValue_Y)))

(fn `UserConstructionScript`)