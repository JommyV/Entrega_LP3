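; AI controller Blueprint that wanders around the world origin by issuing random move orders.
; A looping timer started on BeginPlay fires Move, where a FlipFlop alternates destinations between the positive and negative XY quadrants.
; Only the positive branch passes the controlled pawn to AIMoveTo; the negative branch leaves Pawn unset.
; Each branch prints a freshly randomized number as debug output, separate from the destination values.
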(event `self.ReceiveBeginPlay`
  (`KismetSystemLibrary.K2_SetTimerDelegate` (delegate `Move`) 2.0 true))

(event `Move`
  (bind _returnvalue (`KismetMathLibrary.RandomFloat`))
  (bind _returnvalue_2 (`KismetMathLibrary.RandomFloat`))
  (bind _returnvalue_3 (* _returnvalue 1000.0))
  (bind _returnvalue_4 (* _returnvalue_2 -1000.0))
  (`/Engine/EditorBlueprintResources/StandardMacros.FlipFlop`
    (:`A`
      (`|AIMoveTo` (`self.K2_GetPawn`) (`KismetMathLibrary.MakeVector` (* _returnvalue_2 1000.0) _returnvalue_3) null
        (:`then`
          (`KismetSystemLibrary.PrintString` (`KismetStringLibrary.Conv_DoubleToString` _returnvalue_3)))))
    (:`B`
      (`|AIMoveTo` null (`KismetMathLibrary.MakeVector` _returnvalue_4 (* _returnvalue -1000.0)) null
        (:`then`
          (`KismetSystemLibrary.PrintString` (`KismetStringLibrary.Conv_DoubleToString` _returnvalue_4)))))))

(fn `UserConstructionScript`)